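; Foliage influence Blueprint that feeds the player character's position and motion into the GV_trees_mw_WindParameters material parameter collection, presumably for foliage materials to react to.
; Each tick it writes the lowered character location and both foot socket positions.
; It also writes a lagging trail point that eases toward just behind the player, catching up faster while moving.
; Two speed-based fade scalars are interpolated at different rates.
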(event EventTick
  (params (DeltaSeconds :type Float%20%28single-precision%29))
  (bind _returnvalue (Game|GetPlayerCharacter 0))
  (bind _returnvalue_2 (Game|GetPlayerCharacter 0))
  (bind _returnvalue_3 (Game|GetPlayerCharacter 0))
  (bind _returnvalue_4 (Game|GetPlayerCharacter 0))
  (bind _returnvalue_5 (Utilities|Time|GetWorldDeltaSeconds))
  (bind _returnvalue_6 (Transformation|GetVelocity _returnvalue_4))
  (bind _mesh (Variables|/Script/Engine.Character|GetMesh _returnvalue_3))
  (bind _returnvalue_7 (Math|Vector|VectorGetAbs _returnvalue_6))
  (bind _returnvalue_8 (Math|Vector|VectorLength _returnvalue_7))
  (bind _returnvalue_9 (Math|Float|Clamp(Float) _returnvalue_8 0.0 5e+02))
  (bind _returnvalue_10 (/ _returnvalue_9 5e+02))
  (Utilities|FlowControl|Sequence
    (:then_0
      ;[1 1 1] Player
      (bind _output_get (Variables|Default|SetLocation_Character (Transformation|GetActorLocation _returnvalue_2)))
      (Variables|Default|SetVelocity (Math|Vector|VectorLength (Transformation|GetVelocity _returnvalue_2)))
      (Rendering|Material|SetVectorParameterValue "/Game/GV_FreeShrubsPack/Materials/WindController/GV_trees_mw_WindParameters.GV_trees_mw_WindParameters" "Location" (Math|Conversions|ToLinearColor(Vector) (Math|Vector|MakeVector (.X (Math|Vector|BreakVector _output_get)) (.Y (Math|Vector|BreakVector _output_get)) (+ (.Z (Math|Vector|BreakVector _output_get)) -8e+01))) :!class /Script/Engine.KismetMaterialLibrary))
    (:then_1
      ;[1 1 1] Feet
      (Rendering|Material|SetVectorParameterValue "/Game/GV_FreeShrubsPack/Materials/WindController/GV_trees_mw_WindParameters.GV_trees_mw_WindParameters" "LeftFoot" (Math|Conversions|ToLinearColor(Vector) (Transformation|GetSocketLocation _mesh "foot_l_Socket")) :!class /Script/Engine.KismetMaterialLibrary)
      (Rendering|Material|SetVectorParameterValue "/Game/GV_FreeShrubsPack/Materials/WindController/GV_trees_mw_WindParameters.GV_trees_mw_WindParameters" "RightFoot" (Math|Conversions|ToLinearColor(Vector) (Transformation|GetSocketLocation _mesh "foot_r_Socket")) :!class /Script/Engine.KismetMaterialLibrary))
    (:then_2
      ;[1 1 1] Trail
      (bind _output_get_2 (Variables|Default|SetLocation_Trail (Math|Interpolation|VInterpTo (Variables|Default|GetLocation_Trail) (+ (* (* (Transformation|GetActorForwardVector _returnvalue) -1.0) 5.0) (Transformation|GetActorLocation _returnvalue)) (Utilities|Time|GetWorldDeltaSeconds) (Math|Float|SelectFloat 2.0 0.8 (> (Math|Float|Absolute(Float) (Math|Vector|VectorLength (Transformation|GetVelocity _returnvalue))) 95.0)))))
      (Rendering|Material|SetVectorParameterValue "/Game/GV_FreeShrubsPack/Materials/WindController/GV_trees_mw_WindParameters.GV_trees_mw_WindParameters" "Location_Trail" (Math|Conversions|ToLinearColor(Vector) (Math|Vector|MakeVector (.X (Math|Vector|BreakVector _output_get_2)) (.Y (Math|Vector|BreakVector _output_get_2)) (+ (.Z (Math|Vector|BreakVector _output_get_2)) -4e+01))) :!class /Script/Engine.KismetMaterialLibrary))
    (:then_3
      ;[1 1 1] AnimFade
      (Utilities|FlowControl|Sequence
        (:then_0
          (Variables|Default|SetFadeLong (Math|Interpolation|FInterpTo (Variables|Default|GetFadeLong) _returnvalue_10 _returnvalue_5 1.5))
          (Rendering|Material|SetScalarParameterValue "/Game/GV_FreeShrubsPack/Materials/WindController/GV_trees_mw_WindParameters.GV_trees_mw_WindParameters" "InfluenceFade" (Variables|Default|GetFadeLong) :!class /Script/Engine.KismetMaterialLibrary))
        (:then_1
          (Variables|Default|SetFadeShort (Math|Interpolation|FInterpTo (Variables|Default|GetFadeShort) _returnvalue_10 _returnvalue_5 2.0))
          (Rendering|Material|SetScalarParameterValue "/Game/GV_FreeShrubsPack/Materials/WindController/GV_trees_mw_WindParameters.GV_trees_mw_WindParameters" "InfluenceFadeShort" (Variables|Default|GetFadeShort) :!class /Script/Engine.KismetMaterialLibrary))))))