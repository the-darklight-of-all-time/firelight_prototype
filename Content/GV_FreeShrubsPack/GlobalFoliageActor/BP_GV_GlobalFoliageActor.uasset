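; Global foliage controller actor that drives snow, fall color, leaf brightness and wind for tree materials through the GV_trees_mw_WindParameters material parameter collection.
; UpdateParameters runs from the construction script, BeginPlay and every Tick, pushing the actor's settings into the collection with some remapping.
; Wind direction comes from the actor's yaw, optionally flipped.
; Wind sock and arrow icon components are reoriented to match.
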(event EventBeginPlay
  (Wind|UpdateParameters))

(event EventTick
  (params (DeltaSeconds :type Float%20%28single-precision%29))
  (Wind|UpdateParameters))

(fn ConstructionScript
  (Wind|UpdateParameters))

(fn UpdateParameters
  (bind _icon_sock (Variables|Default|GetIcon_Sock))
  (bind _flip_wind_direction (Variables|Wind(Opaque)|GetFlip%20Wind%20Direction))
  (bind _wind_strength_op (Variables|Wind(Opaque)|GetWind%20Strength%20OP))
  (bind _defaultsceneroot (Variables|Components|GetDefaultSceneRoot))
  (bind _fall_amount (Variables|Season|GetFall%20Amount))
  (bind _returnvalue (Transformation|GetWorldRotation _defaultsceneroot))
  (bind _returnvalue_2 (+ _fall_amount 0.0))
  (bind _returnvalue_3 (/ _wind_strength_op 3e+01))
  (bind _yaw (Math|Rotator|BreakRotator _returnvalue))
  (bind _returnvalue_4 (Math|Rotator|GetRotationXVector _returnvalue))
  (bind _returnvalue_5 (Math|Float|Lerp 1.1 1.1 _returnvalue_3))
  (bind _returnvalue_6 (Math|Conversions|ToLinearColor(Vector) _returnvalue_4))
  (bind _returnvalue_7 (* _returnvalue_4 "-1.000000,-1.000000,-1.000000"))
  (bind _returnvalue_8 (Math|Conversions|ToLinearColor(Vector) _returnvalue_7))
  (Utilities|FlowControl|Sequence
    (:then_0
      ;[1 1 1] Snow
      (Rendering|Material|SetScalarParameterValue "/Game/GV_FreeShrubsPack/Materials/WindController/GV_trees_mw_WindParameters.GV_trees_mw_WindParameters" "Snow Amount" (Variables|Season|GetSnow%20Amount%20Trees) :!class /Script/Engine.KismetMaterialLibrary)
      (Rendering|Material|SetScalarParameterValue "/Game/GV_FreeShrubsPack/Materials/WindController/GV_trees_mw_WindParameters.GV_trees_mw_WindParameters" "Snow Blend Bias" (Variables|Season|GetSnow%20Blend%20Bias%20Trees) :!class /Script/Engine.KismetMaterialLibrary))
    (:then_1
      ;[1 1 1] Material Settings
      (Rendering|Material|SetScalarParameterValue "/Game/GV_FreeShrubsPack/Materials/WindController/GV_trees_mw_WindParameters.GV_trees_mw_WindParameters" "Fall Amount" _returnvalue_2 :!class /Script/Engine.KismetMaterialLibrary)
      (Rendering|Material|SetScalarParameterValue "/Game/GV_FreeShrubsPack/Materials/WindController/GV_trees_mw_WindParameters.GV_trees_mw_WindParameters" "Leaves Brightness" (Variables|Season|GetLeaves%20Brightness) :!class /Script/Engine.KismetMaterialLibrary)
      ;[1 1 1] Wind
      (Rendering|Material|SetScalarParameterValue "/Game/GV_FreeShrubsPack/Materials/WindController/GV_trees_mw_WindParameters.GV_trees_mw_WindParameters" "W Strength Min" (Variables|Wind(Opaque)|GetW%20Strength%20Min) :!class /Script/Engine.KismetMaterialLibrary)
      (Rendering|Material|SetScalarParameterValue "/Game/GV_FreeShrubsPack/Materials/WindController/GV_trees_mw_WindParameters.GV_trees_mw_WindParameters" "W Strength Max" (Variables|Wind(Opaque)|GetW%20Strength%20Max) :!class /Script/Engine.KismetMaterialLibrary)
      (Rendering|Material|SetScalarParameterValue "/Game/GV_FreeShrubsPack/Materials/WindController/GV_trees_mw_WindParameters.GV_trees_mw_WindParameters" "Wind Strength MW Auto Switch" (Variables|Wind(Opaque)|GetW%20Strength%20MW%20Auto%20Switch) :!class /Script/Engine.KismetMaterialLibrary))
    (:then_2
      (Rendering|Material|SetScalarParameterValue "/Game/GV_FreeShrubsPack/Materials/WindController/GV_trees_mw_WindParameters.GV_trees_mw_WindParameters" "Snow" (+ (Variables|Season|GetSnow) _returnvalue_2) :!class /Script/Engine.KismetMaterialLibrary))
    (:then_3
      ;[1 1 1] Flipped Function
      (if _flip_wind_direction
        (Transformation|SetRelativeRotation _icon_sock "0,180.000000, 0" false false)
        (Transformation|SetRelativeLocation _icon_sock "-220.000000, 0, 0" false false) ; fix location of wind sock center to not intersect with the trees
      )
      (if _flip_wind_direction
        (if (< _yaw 0.0)
          (Rendering|Material|SetScalarParameterValue "/Game/GV_FreeShrubsPack/Materials/WindController/GV_trees_mw_WindParameters.GV_trees_mw_WindParameters" "Wind Direction" (+ (/ (+ _yaw 3.6e+02) 3.6e+02) 0.5) :!class /Script/Engine.KismetMaterialLibrary)
          (Rendering|Material|SetVectorParameterValue "/Game/GV_FreeShrubsPack/Materials/WindController/GV_trees_mw_WindParameters.GV_trees_mw_WindParameters" "Wind Direction Vec" _returnvalue_6 :!class /Script/Engine.KismetMaterialLibrary)
          (else
            (Rendering|Material|SetScalarParameterValue "/Game/GV_FreeShrubsPack/Materials/WindController/GV_trees_mw_WindParameters.GV_trees_mw_WindParameters" "Wind Direction" (+ (/ _yaw 3.6e+02) 0.5) :!class /Script/Engine.KismetMaterialLibrary)
            (Rendering|Material|SetVectorParameterValue "/Game/GV_FreeShrubsPack/Materials/WindController/GV_trees_mw_WindParameters.GV_trees_mw_WindParameters" "Wind Direction Vec" _returnvalue_6 :!class /Script/Engine.KismetMaterialLibrary)))
        (elif (< _yaw 0.0)
          (Rendering|Material|SetScalarParameterValue "/Game/GV_FreeShrubsPack/Materials/WindController/GV_trees_mw_WindParameters.GV_trees_mw_WindParameters" "Wind Direction" (/ (+ _yaw 3.6e+02) 3.6e+02) :!class /Script/Engine.KismetMaterialLibrary)
          (Rendering|Material|SetVectorParameterValue "/Game/GV_FreeShrubsPack/Materials/WindController/GV_trees_mw_WindParameters.GV_trees_mw_WindParameters" "Wind Direction Vec" _returnvalue_8 :!class /Script/Engine.KismetMaterialLibrary)
          (else
            (Rendering|Material|SetScalarParameterValue "/Game/GV_FreeShrubsPack/Materials/WindController/GV_trees_mw_WindParameters.GV_trees_mw_WindParameters" "Wind Direction" (/ _yaw 3.6e+02) :!class /Script/Engine.KismetMaterialLibrary)
            (Rendering|Material|SetVectorParameterValue "/Game/GV_FreeShrubsPack/Materials/WindController/GV_trees_mw_WindParameters.GV_trees_mw_WindParameters" "Wind Direction Vec" _returnvalue_8 :!class /Script/Engine.KismetMaterialLibrary))))
      ;[1 1 1] Global Foliage Actor
      (Transformation|SetWorldRotation (Variables|Default|GetIcon_Base) "0, 0, 0" false false)
      (Transformation|SetWorldRotation (Variables|Default|GetIcon_Arrow_Test) (Math|Rotator|MakeRotator 0.0 0.0 (.Yaw (Math|Rotator|BreakRotator (Transformation|GetWorldRotation (Variables|Components|GetDefaultSceneRoot))))) false false)
      ;[1 1 1] Wind
      (Rendering|Material|SetScalarParameterValue "/Game/GV_FreeShrubsPack/Materials/WindController/GV_trees_mw_WindParameters.GV_trees_mw_WindParameters" "Wind Strength OP" (/ (Variables|Wind(Opaque)|GetWind%20Strength%20OP) 3e+01) :!class /Script/Engine.KismetMaterialLibrary)
      (Rendering|Material|SetScalarParameterValue "/Game/GV_FreeShrubsPack/Materials/WindController/GV_trees_mw_WindParameters.GV_trees_mw_WindParameters" "Wind Direction Random" (Variables|Wind(Opaque)|GetWind%20Direction%20Random) :!class /Script/Engine.KismetMaterialLibrary)
      (Rendering|Material|SetScalarParameterValue "/Game/GV_FreeShrubsPack/Materials/WindController/GV_trees_mw_WindParameters.GV_trees_mw_WindParameters" "Wind Direction Random Speed" (* (Variables|Wind(Opaque)|GetWind%20Direction%20Random%20Speed) (Math|Float|Lerp 0.02 0.1 (Math|Float|Sqrt (/ (Variables|Wind(Opaque)|GetWind%20Strength%20OP) 2e+01)))) :!class /Script/Engine.KismetMaterialLibrary)
      (Rendering|Material|SetScalarParameterValue "/Game/GV_FreeShrubsPack/Materials/WindController/GV_trees_mw_WindParameters.GV_trees_mw_WindParameters" "Wind Strength Animation" (Variables|Wind(Opaque)|GetWind%20Strength%20Animation) :!class /Script/Engine.KismetMaterialLibrary)
      (Rendering|Material|SetScalarParameterValue "/Game/GV_FreeShrubsPack/Materials/WindController/GV_trees_mw_WindParameters.GV_trees_mw_WindParameters" "Wind Inertia" (Math|Float|Lerp (* _returnvalue_5 0.7) (* _returnvalue_5 0.25) (Math|Float|Sqrt (Variables|Wind(Opaque)|GetWind%20Direction%20Random%20Speed))) :!class /Script/Engine.KismetMaterialLibrary))))