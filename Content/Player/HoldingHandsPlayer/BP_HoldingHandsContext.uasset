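; Context object for the hand-holding player feature, holding the state of one Leader and Follower pair.
; Initialize assigns both players and returns the context itself, while Clear resets both references to None.
; Getters expose the two players and a hand target location and rotation, which no graph in this Blueprint writes.
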(fn Initialize
  (params (Leader :type BP%20Holding%20Hands%20Player%20Object%20Reference) (Follower :type BP%20Holding%20Hands%20Player%20Object%20Reference))
  (Variables|Default|SetLeader Leader)
  (Variables|Default|SetFollower Follower)
  (return self))

(fn GetPlayers
  (return (Variables|Default|GetLeader) (Variables|Default|GetFollower)))

(fn GetTargetInfo
  (return (Variables|Default|GetHandTargetLocation) (Variables|Default|GetHandTargetRotation)))

(fn Clear
  (Variables|Default|SetLeader 0)
  (Variables|Default|SetFollower 0))