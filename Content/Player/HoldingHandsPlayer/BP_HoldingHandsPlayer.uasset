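; Top-down player Blueprint for a character that faces the mouse cursor and carries a fuel-driven light.
; Tick points the camera boom straight down and offsets the camera by deprojected mouse distance.
; Unless Blue is set, fuel drains every frame, narrowing both spotlight cones.
; Interact messages the interface-implementing actor under the cursor within InteractionRange; hand-holding leader/follower logic is disconnected.
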(event OnComponentBeginOverlap(RightHandArea)
  (params (OverlappedComponent :type Primitive%20Component%20Object%20Reference) (OtherActor :type Actor%20Object%20Reference) (OtherComp :type Primitive%20Component%20Object%20Reference) (OtherBodyIndex :type Integer) (bFromSweep :type Boolean) (SweepResult :type Hit%20Result%20Structure%20%28by%20ref%29))
  ;[1 1 1] disabled for now
)

(event Input|EnhancedActionEvents|EnhancedInputActionIA_Interact
  (params (ActionValue :type Boolean) (ElapsedSeconds :type Float%20%28double-precision%29) (TriggeredSeconds :type Float%20%28double-precision%29) (InputAction :type Input%20Action%20Object%20Reference :default "/Game/ThirdPerson/Input/Actions/IA_Interact.IA_Interact"))
  ;[1 1 1] Interaction, check if implements interface, if cursor is over
  (bind _array_element (Utilities|Array|ForEachLoopwithBreak (Collision|GetOverlappingActors (Variables|Default|GetInteractionRange) "/Script/Engine.Actor" :!class /Script/Engine.PrimitiveComponent) :!label _label)
    (:LoopBody
      (if (and (Utilities|DoesObjectImplementInterface _array_element "/Game/Player/InteractInterface.InteractInterface_C") (== _array_element (.HitActor (Collision|BreakHitResult (.HitResult (Game|Player|GetHitResultUnderCursorbyChannel (Game|GetPlayerController 0) "TraceTypeQuery1" true))))))
        (Class|InteractInterface|Interact(Message) _array_element)
        (goto _label Break)))))

(event EventTick
  (params (DeltaSeconds :type Float%20%28single-precision%29))
  (bind _returnvalue (Transformation|GetActorLocation))
  (bind _returnvalue_2 (Game|GetPlayerController 0))
  (bind _worldlocation (Game|Player|ConvertMouseLocationToWorldSpace _returnvalue_2))
  ;[0.05098 0.05098 0.05098] Player Rotation and Camera Movement
  (Utilities|FlowControl|Sequence
    (:then_0
      (Transformation|SetActorRotation (Math|Rotator|MakeRotator 0.0 0.0 (.yaw (Math|Rotator|FindLookatRotation (Transformation|GetActorLocation) (.Location (Collision|BreakHitResult (.HitResult (Game|Player|GetHitResultUnderCursorbyChannel (Game|GetPlayerController 0) "TraceTypeQuery1" true))))))))
      (Transformation|SetRelativeRotation (Variables|Default|GetCameraBoom) (Math|Rotator|MakeRotator (.yaw (Transformation|GetActorRotation)) -9e+01 0.0) false false)
      (Transformation|SetRelativeLocation (Variables|Default|GetFollowCamera) (Math|Vector|MakeVector -4e+02 0.0 (/ (Math|Float|Sqrt (+ (Math|Float|Square (- (.x _worldlocation) (.x _returnvalue))) (Math|Float|Square (- (.y _worldlocation) (.y _returnvalue))))) 1.05)) false false))
    (:then_1
      ;[1 1 1] Fuel Depletion, Light Settings
      (if (not (Variables|Default|GetBlue))
        (bind _output_get (Variables|Default|SetFuel (Math|Float|Clamp(Float) (- (Variables|Default|GetFuel) 1.0) 0.0 1e+03)))
        (Rendering|Lighting|SetOuterConeAngle (Variables|Default|GetSpotLight1) (Math|Float|Clamp(Float) (* (/ _output_get 1e+03) 7e+01) 0.0 7e+01))
        (Rendering|Lighting|SetOuterConeAngle (Variables|Default|GetSpotLight) (Math|Float|Clamp(Float) (* (/ _output_get 1e+03) 3e+01) 0.0 3e+01))))))

(fn ConstructionScript)