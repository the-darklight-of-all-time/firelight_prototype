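; BP_NPC is an interactable actor that the player destroys to add to their NPC tally.
; Hovering the cursor over its Cube component applies a highlight overlay material, cleared when the cursor leaves.
; Interact starts a destroy montage on the BP_HoldingHandsPlayer mesh and, without waiting for it to finish, plays a sound and spawns an effect.
; It then increments the player's clamped NPCs count and destroys itself.
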(event OnBeginCursorOver(Cube)
  (params (TouchedComponent :type Primitive%20Component%20Object%20Reference))
  (Rendering|Material|SetOverlayMaterial (Variables|Default|GetCube) "/Game/Player/Highlight.Highlight" :!class /Script/Engine.MeshComponent))

(event OnEndCursorOver(Cube)
  (params (TouchedComponent :type Primitive%20Component%20Object%20Reference))
  (Rendering|Material|SetOverlayMaterial (Variables|Default|GetCube) 0 :!class /Script/Engine.MeshComponent))

(event EventInteract
  (bind _asbp_holding_hands_player (Utilities|Casting|CastToBP_HoldingHandsPlayer (Game|GetPlayerCharacter 0)))
  (Animation|Montage|PlayMontage (Variables|/Script/Engine.Character|GetMesh _asbp_holding_hands_player) "/Game/Player/Anims/MF_Destroy_Montage.MF_Destroy_Montage"
    (:then
      (Audio|PlaySound2D "/Game/Player/Music_SFX/destroy_Cue.destroy_Cue" 1.0 1.0 0.0 0 0)
      (Niagara|SpawnSystematLocation "/Game/Player/Particles/Destroy.Destroy" (Transformation|GetActorLocation))
      (Variables|/Game/Player/HoldingHandsPlayer/BP_HoldingHandsPlayer.BP_HoldingHandsPlayer_C|SetNPCs _asbp_holding_hands_player (Math|Integer|Clamp(Integer) (+ (Variables|/Game/Player/HoldingHandsPlayer/BP_HoldingHandsPlayer.BP_HoldingHandsPlayer_C|GetNPCs _asbp_holding_hands_player) 1) 0 12))
      (Actor|DestroyActor))))

(fn ConstructionScript)