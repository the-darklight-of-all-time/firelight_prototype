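; BP_NPC_NONFUNCTIONAL is an interactable NPC character that highlights its cube under the cursor.
; Each tick it writes the player's location to the FollowLocation blackboard key for its AI.
; Interact plays a destroy montage on the player, increments their clamped NPC count, then calls Activate on CharacterMovement.
; That component's activation event serves as the trigger for the destroy sound and effect, though the actor itself is never destroyed here.
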(event OnBeginCursorOver(Cube)
  (params (TouchedComponent :type Primitive%20Component%20Object%20Reference))
  (Rendering|Material|SetOverlayMaterial (Variables|Default|GetCube) "/Game/Player/Highlight.Highlight" :!class /Script/Engine.MeshComponent))

(event OnEndCursorOver(Cube)
  (params (TouchedComponent :type Primitive%20Component%20Object%20Reference))
  (Rendering|Material|SetOverlayMaterial (Variables|Default|GetCube) 0 :!class /Script/Engine.MeshComponent))

(event OnComponentActivated(CharacterMovement)
  (params (Component :type Actor%20Component%20Object%20Reference) (bReset :type Boolean))
  (Audio|PlaySound2D "/Game/Player/Music_SFX/destroy_Cue.destroy_Cue" 1.0 1.0 0.0 0 0)
  (Niagara|SpawnSystematLocation "/Game/Player/Particles/Destroy.Destroy" (Transformation|GetActorLocation)))

(event EventTick
  (params (DeltaSeconds :type Float%20%28single-precision%29))
  (bind _asbp_holding_hands_player (Utilities|Casting|CastToBP_HoldingHandsPlayer (Game|GetPlayerCharacter 0)))
  (AI|Components|Blackboard|SetValueasVector (AI|GetBlackboard 0) (Variables|Default|GetFollowLocation) (Transformation|GetActorLocation _asbp_holding_hands_player)))

(event EventInteract
  (bind _asbp_holding_hands_player (Utilities|Casting|CastToBP_HoldingHandsPlayer (Game|GetPlayerCharacter 0)))
  (Animation|Montage|PlayMontage (Variables|/Script/Engine.Character|GetMesh _asbp_holding_hands_player) "/Game/Player/Anims/MF_Destroy_Montage.MF_Destroy_Montage"
    (:then
      (Variables|/Game/Player/HoldingHandsPlayer/BP_HoldingHandsPlayer.BP_HoldingHandsPlayer_C|SetNPCs _asbp_holding_hands_player (Math|Float|Clamp(Float) (+ (Variables|/Game/Player/HoldingHandsPlayer/BP_HoldingHandsPlayer.BP_HoldingHandsPlayer_C|GetNPCs _asbp_holding_hands_player) 1.0) 0.0 12.0))
      (Components|Activation|Activate (Variables|Character|GetCharacterMovement) false))))

(fn ConstructionScript)