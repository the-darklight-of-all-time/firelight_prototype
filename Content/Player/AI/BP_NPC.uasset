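; BP_NPC is an interactable NPC that follows the player once recruited.
; It shows a highlight overlay under the cursor until Interact plays reaching-out montages on both characters, raises the player's capped NPC count and triggers a sound, particle burst, spotlight and Niagara effect.
; Tick issues AIMoveTo toward the player after interaction and polls the player's IsBlue flag to turn the light and flame blue.
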(event OnBeginCursorOver(Mesh)
  (params (TouchedComponent :type Primitive%20Component%20Object%20Reference))
  (if (not (Variables|Default|GetInteracted))
    (Rendering|Material|SetOverlayMaterial (Variables|Character|GetMesh) "/Game/Player/Highlight.Highlight" :!class /Script/Engine.MeshComponent)))

(event OnEndCursorOver(Mesh)
  (params (TouchedComponent :type Primitive%20Component%20Object%20Reference))
  (Rendering|Material|SetOverlayMaterial (Variables|Character|GetMesh) 0 :!class /Script/Engine.MeshComponent))

(event EventBeginPlay
  (Rendering|SetVisibility (Variables|Default|GetSpotLight) false false))

(event Collision|EventActorBeginOverlap
  (params (OtherActor :type Actor%20Object%20Reference)))

(event EventTick
  (params (DeltaSeconds :type Float%20%28single-precision%29))
  (bind _returnvalue (Game|GetPlayerCharacter 0))
  (if (Variables|Default|GetInteracted)
    (AI|AIMoveTo self (Transformation|GetActorLocation _returnvalue) _returnvalue 1.5e+02 false
      (:then
        _)))
  (bind _asbp_holding_hands_player (Utilities|Casting|CastToBP_HoldingHandsPlayer (Game|Player|GetPlayerPawn 0)))
  (if (Variables|/Game/Player/HoldingHandsPlayer/BP_HoldingHandsPlayer.BP_HoldingHandsPlayer_C|GetIsBlue _asbp_holding_hands_player)
    (Rendering|Components|Light|SetLightColor (Variables|Default|GetSpotLight) "(R=0.000000,G=0.478431,B=1.000000,A=1.000000)" true)
    (Class|NiagaraComponent|SetAsset (Variables|Default|GetNiagara) "/Game/F_FreeFlameFx_Pack/FX/NS_Flame_8_Torch_Blue.NS_Flame_8_Torch_Blue" true)))

(event EventInteract
  (if (not (Variables|Default|GetInteracted))
    (bind _asbp_holding_hands_player (Utilities|Casting|CastToBP_HoldingHandsPlayer (Game|GetPlayerCharacter 0)))
    (Animation|Montage|PlayMontage (Variables|/Script/Engine.Character|GetMesh _asbp_holding_hands_player) "/Game/Player/Anims/Reaching_Out_Montage.Reaching_Out_Montage" 2.0
      (:then
        (Animation|Montage|PlayMontage (Variables|Character|GetMesh) "/Game/Player/Anims/Reaching_Out1_Montage.Reaching_Out1_Montage" 2.0
          (:then
            (Variables|/Game/Player/HoldingHandsPlayer/BP_HoldingHandsPlayer.BP_HoldingHandsPlayer_C|SetNPCs _asbp_holding_hands_player (Math|Float|Clamp(Float) (+ (Variables|/Game/Player/HoldingHandsPlayer/BP_HoldingHandsPlayer.BP_HoldingHandsPlayer_C|GetNPCs _asbp_holding_hands_player) 1.0) 0.0 12.0))
            (Audio|PlaySound2D "/Game/Player/Music_SFX/destroy_Cue.destroy_Cue" 1.0 1.0 0.0 0 0)
            (Niagara|SpawnSystematLocation "/Game/Player/Particles/Destroy.Destroy" (Transformation|GetActorLocation))
            (Variables|Default|SetInteracted true)
            (Rendering|SetVisibility (Variables|Default|GetSpotLight) true false)
            (Components|Activation|Activate (Variables|Default|GetNiagara) false)))))))

(fn ConstructionScript)